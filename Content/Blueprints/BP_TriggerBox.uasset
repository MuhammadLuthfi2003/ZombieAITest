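; BP_TriggerBox is a configurable trigger volume for a course that compares Behavior Tree and FSM zombies.
; On overlap, flags let it set zombie state, change walk speed while disabling attacks, or act as a finish line printing transition times.
; Other flags update the speed of every Car cached at BeginPlay or activate a linked platform, whatever actor overlaps.
; The FSM finish readout waits five seconds and adds game time.
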(event `self.ReceiveBeginPlay`
  (bind _outactors (`GameplayStatics.GetAllActorsOfClass` "/Game/Car/Car.Car_C"))
  (set `self.CarRefrences` _outactors))

(event `self.ReceiveActorBeginOverlap`
  (params (OtherActor :type "Actor Object Reference"))
  (bind _returnvalue (`GameplayStatics.GetObjectClass` OtherActor))
  (bind _returnvalue_2 (`GameplayStatics.GetObjectClass` OtherActor))
  (bind _returnvalue_3 (`GameplayStatics.GetObjectClass` OtherActor))
  (bind _returnvalue_4 (`GameplayStatics.GetObjectClass` OtherActor))
  (bind _platform (`self.Platform`))
  (`|ExecutionSequence`
    (:`then_0`
      (if (`self.ChangeState?`)
        (if (or (== _returnvalue_2 "/Game/Zombie/Zombie_BT.Zombie_BT_C") (== _returnvalue_2 "/Game/Zombie/Zombie_FSM.Zombie_FSM_C"))
          (if (== _returnvalue_3 "/Game/Zombie/Zombie_BT.Zombie_BT_C")
            (bind _aszombie_bt (cast `/Game/Zombie/Zombie_BT` OtherActor))
            (`/Game/Zombie/Zombie_BT.SetState` _aszombie_bt (`self.StateToChangeInto`))
            (elif (== _returnvalue_3 "/Game/Zombie/Zombie_FSM.Zombie_FSM_C")
              (bind _aszombie_fsm (cast `/Game/Zombie/Zombie_FSM` OtherActor))
              (`/Game/Zombie/Zombie_FSM.SetState` _aszombie_fsm (`self.StateToChangeInto`)))))))
    (:`then_1`
      (if (`self.ChangeActorSpeed?`)
        (if (== _returnvalue_4 "/Game/Zombie/Zombie_BT.Zombie_BT_C")
          (bind _aszombie_bt_2 (cast `/Game/Zombie/Zombie_BT` OtherActor))
          (set `CharacterMovementComponent.MaxWalkSpeed` (`self.NewActorSpeed`) (`Character.CharacterMovement` _aszombie_bt_2))
          (set `/Game/Zombie/Zombie_BT.CanAttack` false _aszombie_bt_2)
          (elif (== _returnvalue_4 "/Game/Zombie/Zombie_FSM.Zombie_FSM_C")
            (bind _aszombie_fsm_2 (cast `/Game/Zombie/Zombie_FSM` OtherActor))
            (set `CharacterMovementComponent.MaxWalkSpeed` (`self.NewActorSpeed`) (`Character.CharacterMovement` _aszombie_fsm_2))
            (set `/Game/Zombie/Zombie_FSM.CanAttack` false _aszombie_fsm_2)))))
    (:`then_2`
      (if (`self.ChangeCarSpeed?`)
        (for _array_element (`self.CarRefrences`)
          (set `/Game/Car/Car.CarSpeed` (`self.NewCarSpeed`) _array_element))))
    (:`then_3`
      (if (`self.isFinishLine?`)
        (if (== _returnvalue "/Game/Zombie/Zombie_BT.Zombie_BT_C")
          (`KismetSystemLibrary.PrintString` "BT Reaction Time:" true true (struct :`R` 1.0 :`B` 0.042414 :`A` 1.0) 100.0)
          (bind _aszombie_bt_3 (cast `/Game/Zombie/Zombie_BT` OtherActor))
          (for _array_element_2 (`/Game/Zombie/Zombie_BT.TransitionTimeList` _aszombie_bt_3)
            (`KismetSystemLibrary.PrintString` (`KismetStringLibrary.Conv_DoubleToString` _array_element_2) true true (struct :`R` 1.0 :`B` 0.042414 :`A` 1.0) 100.0))
          (elif (== _returnvalue "/Game/Zombie/Zombie_FSM.Zombie_FSM_C")
            (`KismetSystemLibrary.Delay` 5.0)
            (`KismetSystemLibrary.PrintString` (`KismetStringLibrary.Concat_StrStr` "FSM Finish Time:" "" (`KismetStringLibrary.Conv_DoubleToString` (`KismetSystemLibrary.GetGameTimeInSeconds`))) true true (struct :`R` 1.0 :`G` 0.886856 :`A` 1.0) 100.0)
            (bind _aszombie_fsm_3 (cast `/Game/Zombie/Zombie_FSM` OtherActor))
            (for _array_element_3 (`/Game/Zombie/Zombie_FSM.TransitionTimeLists` _aszombie_fsm_3)
              (`KismetSystemLibrary.PrintString` (`KismetStringLibrary.Conv_DoubleToString` _array_element_3) true true (struct :`R` 0.93004 :`G` 1.0 :`A` 1.0) 100.0))))))
    (:`then_4`
      (if (`self.ActivatePlatform?`)
        (`/Engine/EditorBlueprintResources/StandardMacros.IsValid` _platform
          (:`Is Valid`
            (`/Game/MovingPlatform.ActivatePlatform` _platform)))))))

(fn `UserConstructionScript`)